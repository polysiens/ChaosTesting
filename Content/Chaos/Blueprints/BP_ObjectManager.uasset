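; Object manager that provides shared object data actors and decides when a virtual mesh snaps onto nearby Geometry Collection objects by their hinges.
; Caches one data actor per class, spawned far below the world.
; Box-overlaps Destructibles, then compares same-index hinge volumes by distance, Grabber/Attacher pairing and main-axis size.
; A match returns a locked transform built from the hinge's relative transform and the target's root; debug boxes show hinge positions.
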(fn `CheckConnectionsVirtualMesh`
  (params (ObjectData_Reference :type "Actor Object Reference") (VirtualMesh :type "PrimitiveComponent Object Reference") (OriginalObject :type "GeometryCollectionActor Object Reference") (LocationCheckTrace :type "Vector Structure"))
  (returns (`VirtualMeshLocked?` :type Boolean) (LockedLocation :type "Transform Structure"))
  (locals (CurrentIndex :type Integer) (VMBoxExtent :type "Array of Vector Structure") (OvelappedBoxExtent :type "Array of Vector Structure") (OverlappedAttributes :type "Array of /Game/Chaos/Data/ST_Attributes Structure") (VMAttributes :type "Array of /Game/Chaos/Data/ST_Attributes Structure"))
  (bind _currentindex (`local.CurrentIndex`))
  (bind _output_attributes (break `/Game/Chaos/Data/ST_Attributes` (`|GetArrayItem` (`local.VMAttributes`) (`local.CurrentIndex`))))
  (bind _output_attributes_2 (break `/Game/Chaos/Data/ST_Attributes` (`|GetArrayItem` (`local.OverlappedAttributes`) (`local.CurrentIndex`))))
  (bind _returnvalue (`KismetArrayLibrary.Array_Contains` _output_attributes_2 "Grabber"))
  (bind _mainaxissize (`self.GetMainAxisHinge` (`|GetArrayItem` (`local.OvelappedBoxExtent`) (`local.CurrentIndex`)) (`|GetArrayItem` (`local.OverlappedAttributes`) (`local.CurrentIndex`))))
  (bind _mainaxissize_2 (`self.GetMainAxisHinge` (`|GetArrayItem` (`local.VMBoxExtent`) (`local.CurrentIndex`)) (`|GetArrayItem` (`local.VMAttributes`) (`local.CurrentIndex`))))
  (bind _outcomponents (`KismetSystemLibrary.BoxOverlapComponents` LocationCheckTrace (`.BoxExtent` (`KismetSystemLibrary.GetComponentBounds` VirtualMesh)) (`|MakeArray` "ObjectTypeQuery6" :!type "EObjectTypeQuery Enum")))
  (for _array_element _outcomponents
    (bind _returnvalue_2 (`ActorComponent.GetOwner` _array_element))
    (if (== _returnvalue_2 (`local.OriginalObject`))
      (`KismetSystemLibrary.PrintString` "ORIGINAL OBJECT" true true (struct :`R` 1.0 :`G` 0.5 :`A` 1.0))
      (else
        (bind _objectdata (message `/Game/Chaos/Blueprints/Interfaces/BPI_Objects.GetObjectDataReference` _returnvalue_2))
        (bind (_hinge_volumes _hinge_constraints _couplinggroups _attributes _hinge_boxextent) (message `/Game/Chaos/Blueprints/Interfaces/BPI_Objects.GetHingeData` _objectdata))
        (set `local.OvelappedBoxExtent` _hinge_boxextent)
        (set `local.OverlappedAttributes` _attributes)
        (bind (_hinge_volumes_2 _hinge_constraints_2 _couplinggroups_2 _attributes_2 _hinge_boxextent_2) (message `/Game/Chaos/Blueprints/Interfaces/BPI_Objects.GetHingeData` ObjectData_Reference))
        (set `local.VMBoxExtent` _hinge_boxextent_2)
        (set `local.VMAttributes` _attributes_2)
        (for (_ _array_index) _hinge_volumes_2
          (set `local.CurrentIndex` _array_index)
          (bind _output (`|GetArrayItem` _hinge_volumes_2 _currentindex))
          (bind _returnvalue_3 (`GeometryCollectionComponent.GetRootCurrentTransform` (`GeometryCollectionActor.GeometryCollectionComponent` (cast `GeometryCollectionActor` (`ActorComponent.GetOwner` _array_element) :!pure true))))
          (bind (_locationmatched_ _component1_location _component2_location) (`self.CheckHingeLocation` (`self.GetTransform` (`ActorComponent.GetOwner` (`local.VirtualMesh`))) _output (`|GetArrayItem` _hinge_volumes _currentindex) _returnvalue_3))
          (`KismetSystemLibrary.DrawDebugBox` _component1_location (0.0 0.0 0.0) (struct :`G` 0.159579 :`B` 1.0 :`A` 1.0) (struct) 0.1 1.0)
          (`KismetSystemLibrary.DrawDebugBox` _component2_location (0.3 0.3 0.3) (struct :`R` 1.0 :`B` 0.065304 :`A` 1.0) (struct) 0.1 1.0)
          (if _locationmatched_
            (if (or (and _returnvalue (`KismetArrayLibrary.Array_Contains` _output_attributes "Attacher")) (and (`KismetArrayLibrary.Array_Contains` _output_attributes_2 "Attacher") (`KismetArrayLibrary.Array_Contains` _output_attributes "Grabber")))
              (if (select `bool` _returnvalue :`false` (>= (+ _mainaxissize_2 0.05) _mainaxissize) :`true` (>= (+ _mainaxissize 0.05) _mainaxissize_2))
                (return true (`KismetMathLibrary.ComposeTransforms` (`SceneComponent.GetRelativeTransform` _output) _returnvalue_3)))
              (else
                (`KismetSystemLibrary.PrintString` "NOT COMPATIBLE"))))))))
  (return false))

(fn `CheckHingeLocation`
  (params (Component1_Transform :type "Transform Structure") (Component1 :type "SceneComponent Object Reference") (Component2 :type "SceneComponent Object Reference") (Component2_Transform :type "Transform Structure"))
  (returns (`LocationMatched?` :type Boolean) (Component1_Location :type "Vector Structure") (Component2_Location :type "Vector Structure"))
  (bind _returnvalue (+ (.location Component1_Transform) (`KismetMathLibrary.GreaterGreater_VectorRotator` (`SceneComponent.RelativeLocation` Component1) (.rotation Component1_Transform))))
  (bind _returnvalue_2 (+ (`KismetMathLibrary.GreaterGreater_VectorRotator` (`SceneComponent.RelativeLocation` Component2) (.rotation Component2_Transform)) (.location Component2_Transform)))
  (return (< (`KismetMathLibrary.Vector_Distance` _returnvalue _returnvalue_2) 2.2) _returnvalue _returnvalue_2))

(fn `GetMainAxisHinge`
  (params (BoxExtent :type "Vector Structure") (Attributes :type "/Game/Chaos/Data/ST_Attributes Structure"))
  (returns (MainAxisSize :type "Float (double-precision)"))
  (return (select `int` (`KismetStringLibrary.Conv_StringToInt` (`|GetArrayItem` Attributes_Values_19_E203258342EEA1890EA0D7A1D327BA7F (`KismetArrayLibrary.Array_Find` Attributes_Attributes_7_917776F64D9F03E16829F28485763C3B "RotateAroundAxis"))) :`0` BoxExtent_X :`1` BoxExtent_Y :`2` BoxExtent_Z)))

(fn `Spawn Object Data Actor`
  (params (ObjectDataClass :type "Actor Class Reference"))
  (returns (SpawnedActor :type "Actor Object Reference"))
  (bind (_value _returnvalue) (`BlueprintMapLibrary.Map_Find` (`self.ReferenceObjects`) (`local.ObjectDataClass`)))
  (if _returnvalue
    (return _value)
    (else
      (bind _returnvalue_2 (`|SpawnActorFromClass` ObjectDataClass (`KismetMathLibrary.MakeTransform` (0.0 0.0 -99999.0)) "AlwaysSpawn" "MultiplyWithRoot" null null))
      (`BlueprintMapLibrary.Map_Add` (`self.ReferenceObjects`) ObjectDataClass _returnvalue_2)
      (return _returnvalue_2))))

(fn `UserConstructionScript`)