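; BP_ObjectGeneric is a generic actor in the Chaos folder that can gain a mesh component at runtime.
; AddComponentClass adds a component of the given class, then switches on ClassName to cast it and assign the supplied asset as a static mesh, skeletal mesh or Geometry Collection.
; It returns the new component; the event graph and construction script are empty.
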(fn `AddComponentClass`
  (params (Class :type "ActorComponent Class Reference") (ClassName :type "/Game/Chaos/Data/ComponentType_Enum Enum" :default "NewEnumerator0") (Object :type "Object Object Reference"))
  (returns (AddedComponent :type "ActorComponent Object Reference"))
  (bind _returnvalue (`|AddComponentByClass` Class))
  (switch `/Game/Chaos/Data/ComponentType_Enum` ClassName
    (:`NewEnumerator0`
      (`StaticMeshComponent.SetStaticMesh` (cast `StaticMeshComponent` _returnvalue :!pure true) (cast `StaticMesh` (`local.Object`) :!pure true))
      (return _returnvalue))
    (:`NewEnumerator1`
      (bind _asskeletal_mesh_component (cast `SkeletalMeshComponent` _returnvalue))
      (set `SkeletalMeshComponent.SkeletalMeshAsset` (cast `SkeletalMesh` (`local.Object`) :!pure true) _asskeletal_mesh_component)
      (return _returnvalue))
    (:`NewEnumerator2`
      (bind _asgeometry_collection_component (cast `GeometryCollectionComponent` _returnvalue))
      (`GeometryCollectionComponent.SetRestCollection` _asgeometry_collection_component (cast `GeometryCollection` (`local.Object`) :!pure true) true)
      (return _returnvalue))))

(fn `UserConstructionScript`)